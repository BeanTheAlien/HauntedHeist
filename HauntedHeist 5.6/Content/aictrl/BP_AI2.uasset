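; BP_AI2 is an AI Blueprint that provides an attack, damaging the player passed to it as a target.
; Its Attack event runs a debug-drawn sphere trace for Pawns, centered on the target's own location rather than the AI's.
; When a hit matches the target and carries the "player" tag, it casts to Player, decrements Health, calls PlayerHealthUpdate and stops looping.
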(event `/Game/aictrl/BPI_Murder.Attack`
  (params (tg :type "Actor Object Reference"))
  (bind _returnvalue (`self.K2_GetActorLocation` tg))
  (bind (_outhits _returnvalue_2) (`KismetSystemLibrary.SphereTraceMultiForObjects` :`Start` _returnvalue :`End` _returnvalue :`Radius` 200.0 :`ObjectTypes` (`|MakeArray` "ObjectTypeQuery3" :!type "EObjectTypeQuery Enum") :`DrawDebugType` "ForDuration"))
  (if _returnvalue_2
    (for _array_element _outhits
      (bind (_bblockinghit _binitialoverlap _time _distance _location _impactpoint _normal _impactnormal _physmat _hitactor) (`GameplayStatics.BreakHitResult` _array_element))
      (if (== _hitactor tg)
        (if (`self.ActorHasTag` _hitactor "player")
          (bind _asplayer (cast `/Game/FirstPerson/Blueprints/Player` _hitactor))
          (`/Engine/EditorBlueprintResources/StandardMacros.DecrementInt` (`/Game/FirstPerson/Blueprints/Player.health` _asplayer)
            (:`  `
              (`/Game/FirstPerson/Blueprints/Player.PlayerHealthUpdate` _asplayer)
              (break))))))))

(fn `UserConstructionScript`)