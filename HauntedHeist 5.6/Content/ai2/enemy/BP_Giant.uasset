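; Giant enemy character that adds its own music, voice sounds and knockback attack to a parent enemy class.
; Starts looping-timer countdown and background music on spawn, fading the music out on ragdoll.
; Tick plays random yells, throttled by that countdown; hurt stops movement, and hurt, attack and death play random sounds.
; Attacking launches player pawn 0 along the giant's forward vector with randomized speed and lift.
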(event `dec`
  (`/Engine/EditorBlueprintResources/StandardMacros.DecrementInt` (`self.lastnoise`)))

(event `self.ReceiveBeginPlay`
  (`parent.ReceiveBeginPlay`)
  (`KismetSystemLibrary.K2_SetTimerDelegate` (delegate `dec`) 1.0 true true)
  (bind _returnvalue (`GameplayStatics.SpawnSound2D` (`self.bgm`) 1.0 1.0 0.0 null false false))
  (set `self.bgmhandle` _returnvalue))

(event `self.ReceiveTick`
  (params (DeltaSeconds :type "Float (single-precision)"))
  (`parent.ReceiveTick` DeltaSeconds)
  (if (and (<= (`KismetMathLibrary.RandomIntegerInRange` 0 100) 65) (<= (`self.lastnoise`) 0))
    (`self.Rand` (`self.tyell`))
    (set `self.lastnoise` 5)))

(event `Rand`
  (params (aud :type "Array of SoundWave Object Reference"))
  (`GameplayStatics.PlaySoundAtLocation` (`KismetArrayLibrary.Array_Random` aud) (`self.K2_GetActorLocation`) (struct) 1.0 1.0 0.0 null null null null))

(event `self.OnHurt`
  (`MovementComponent.StopMovementImmediately` (`self.CharacterMovement`))
  (`self.Rand` (`self.thurt`)))

(event `self.ragdoll`
  (`parent.ragdoll`)
  (`self.Rand` (`self.tdeath`))
  (`AudioComponent.FadeOut` (`self.bgmhandle`) 5.0 0.0 "Linear"))

(event `self.OnAttack`
  (`self.Rand` (`self.tpunch`))
  (bind _asplayer (cast `/Game/FirstPerson/Blueprints/Player` (`GameplayStatics.GetPlayerPawn` 0)))
  (`self.throw` _asplayer))

(event `throw`
  (params (char :type "Character Object Reference"))
  (bind _out (`self.getforwardvel`))
  (`self.LaunchCharacter` char _out true true))

(fn `getforwardvel`
  (returns (out :type "Vector Structure"))
  (return (+ (* (`KismetMathLibrary.GetForwardVector` (`self.K2_GetActorRotation`)) (`KismetMathLibrary.RandomFloatInRange` 1400.0 1500.0)) (`KismetMathLibrary.MakeVector` 0.0 0.0 (`KismetMathLibrary.RandomFloatInRange` 500.0 750.0)))))

(fn `UserConstructionScript`
  (`parent.UserConstructionScript`))