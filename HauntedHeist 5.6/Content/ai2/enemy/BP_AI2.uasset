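; BP_AI2 is an enemy character with health, an attack and a ragdoll death that rewards the player.
; Hurt subtracts damage, then either ragdolls the enemy or fires OnHurt, and death adds Value to player Tokens once.
; Attack sphere-traces around the target's own location, docking one health if it is player-tagged, otherwise firing OnAttackFailed.
; OnHurt, OnAttack and OnAttackFailed are empty hooks, and no movement or targeting logic lives here.
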(event `OnHurt`)

(event `hurt`
  (params (dmg :type "Float (double-precision)"))
  (bind _output_get (set `self.health` (- (`self.health`) dmg)))
  (if (<= _output_get 0.0)
    (`self.ragdoll`)
    (else
      (`self.OnHurt`)
      (`KismetSystemLibrary.PrintString` (`KismetStringLibrary.Conv_DoubleToString` _output_get)))))

(event `/Game/ai2/BPI_Murder.Attack`
  (params (tg :type "Actor Object Reference"))
  (bind _returnvalue (`self.K2_GetActorLocation` tg))
  (bind (_outhits _returnvalue_2) (`KismetSystemLibrary.SphereTraceMultiForObjects` _returnvalue _returnvalue 200.0 (`|MakeArray` "ObjectTypeQuery3" :!type "EObjectTypeQuery Enum")))
  (if _returnvalue_2
    (for _array_element _outhits
      (bind (_bblockinghit _binitialoverlap _time _distance _location _impactpoint _normal _impactnormal _physmat _hitactor _hitcomponent) (`GameplayStatics.BreakHitResult` _array_element))
      (if (== _hitactor tg)
        (if (`self.ActorHasTag` _hitactor "player")
          (bind _asplayer (cast `/Game/FirstPerson/Blueprints/Player` _hitactor))
          (`/Engine/EditorBlueprintResources/StandardMacros.DecrementInt` (`/Game/FirstPerson/Blueprints/Player.health` _asplayer)
            (:`  `
              (`/Game/FirstPerson/Blueprints/Player.PlayerHealthUpdate` _asplayer)
              (`self.OnAttack`)
              (break)))
          (else
            (`self.OnAttackFailed` _hitactor _hitcomponent)))))))

(event `ragdoll`
  (bind _mesh (`self.Mesh`))
  (if (`self.alive`)
    (`PrimitiveComponent.SetSimulatePhysics` _mesh true)
    (`SkeletalMeshComponent.SetPhysicsBlendWeight` _mesh 1.0)
    (`ActorComponent.K2_DestroyComponent` (`self.CapsuleComponent`))
    (set `self.alive` false)
    (bind _asplayer (cast `/Game/FirstPerson/Blueprints/Player` (`GameplayStatics.GetPlayerPawn` 0)))
    (set `/Game/FirstPerson/Blueprints/Player.tokens` (+ (`/Game/FirstPerson/Blueprints/Player.tokens` _asplayer) (`self.value`)) _asplayer)))

(event `OnAttack`)

(event `OnAttackFailed`
  (params (actor :type "Actor Object Reference") (comp :type "PrimitiveComponent Object Reference")))

(fn `UserConstructionScript`)